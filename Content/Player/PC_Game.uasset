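; PC_Game is the in-game player controller that sets game-only input and drives periodic auto-saving.
; On BeginPlay it hides the cursor, asks the game instance to send an info message and starts a looping timer that triggers auto-saves every few seconds.
; Saving is delegated to the game instance.
; Debug keys trigger a non-auto save, open the main menu, delete the save slots or print the first slot's auto-save list.
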(event Custom|AutoSave
  (Utilities|Time|SetTimerbyEvent (delegate Custom|TriggerSave) 3.0 true))

(event Custom|TriggerSave
  (Class|BISystem|StartSaveGame(Message) (Game|GetGameInstance) true))

(event EventBeginPlay
  (Input|SetInputModeGameOnly self true)
  (Variables|Default|SetbShowMouseCursor false)
  (Class|BISystem|SendInfo(Message) (Game|GetGameInstance))
  (CallFunction|AutoSave))

(event Input|KeyboardEvents|DebugKey1
  (params (Key :type Key%20Structure :default "None") (ActionValue :type Input%20Action%20Value%20Structure))
  (:Pressed
    (Class|BISystem|StartSaveGame(Message) (Game|GetGameInstance) false)))

(event Input|KeyboardEvents|DebugKey2
  (params (Key :type Key%20Structure :default "None") (ActionValue :type Input%20Action%20Value%20Structure))
  (:Pressed
    (Game|OpenLevel(byObjectReference) "/Game/Maps/MainMenu.MainMenu")))

(event Input|KeyboardEvents|DebugKey3
  (params (Key :type Key%20Structure :default "None") (ActionValue :type Input%20Action%20Value%20Structure))
  (:Pressed
    (SaveGame|DeleteGameinSlot "Slot1")
    (SaveGame|DeleteGameinSlot "Slot2")
    (SaveGame|DeleteGameinSlot "Slot3")
    (Development|PrintString "Deleted")))

(event Input|KeyboardEvents|DebugKey4
  (params (Key :type Key%20Structure :default "None") (ActionValue :type Input%20Action%20Value%20Structure))
  (:Pressed
    (bind _returnvalue (SaveGame|LoadGamefromSlot "Slot1"))
    (bind _savegame (Class|BISaveFile|GetSGFile(Message) _returnvalue))
    (for _array_element (Variables|/Game/SaveGame/SG_SaveFile.SG_SaveFile_C|GetAutoSaves _savegame)
      (Development|PrintString _array_element))))

(fn ConstructionScript)